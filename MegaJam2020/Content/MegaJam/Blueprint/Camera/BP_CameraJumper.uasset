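; BP_CameraJumper is the gameplay camera actor that follows the bubble jumper character along a camera track.
; On BeginPlay it registers itself with the bubble-jumping GameState and caches the first BP_CameraTrack and the player pawn.
; Each tick the track supplies a position and rotation; the camera takes that pitch and yaw with zero roll, then shifts from the track point toward the player by a weighted share of their distance.
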(event EventBeginPlay
  (Variables|/Game/MegaJam/Blueprint/GameData/GameState_BubbleJumping.GameState_BubbleJumping_C|SetCameraJumper (.AsGame%20State%20Bubble%20Jumping (Utilities|Casting|CastToGameState_BubbleJumping (Game|GetGameState))) self)
  (bind _outactors (Actor|GetAllActorsOfClass "/Game/MegaJam/Blueprint/Camera/BP_CameraTrack.BP_CameraTrack_C"))
  (Variables|Default|SetCameraTrack (Utilities|Array|Get(acopy) _outactors))
  (Variables|Default|SetBubbleJumper (.AsBP%20Bubble%20Jumper%20Character (Utilities|Casting|CastToBP_BubbleJumperCharacter (Game|Player|GetPlayerPawn 0)))))

(event EventTick
  (params (DeltaSeconds :type Float%20%28single-precision%29))
  (bind _bubblejumper (Variables|Default|GetBubbleJumper))
  (bind _cameratrack (Variables|Default|GetCameraTrack))
  (bind _returnvalue (Transformation|GetActorLocation _bubblejumper))
  (bind _bubblejumper_2 (Variables|Default|GetBubbleJumper)
    (:then
      (bind _returnvalue_2 (Default|GetPlayerLocationonTrack _cameratrack))
      (bind _returnvalue_3 (Default|GetCameraRotation _cameratrack _returnvalue_2 _bubblejumper_2))
      (Transformation|SetActorRotation (Math|Rotator|MakeRotator 0.0 (.Pitch (Math|Rotator|BreakRotator _returnvalue_3)) (.Yaw (Math|Rotator|BreakRotator _returnvalue_3))))
      (Transformation|SetActorLocation (+ _returnvalue_2 (* (Math|Vector|Normalize (- _returnvalue _returnvalue_2)) (* (Math|Vector|Distance(Vector) _returnvalue_2 _returnvalue) (Variables|Default|GetOffsetWeight)))) false false))
    (:else)))

(fn ConstructionScript)