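; BP_CameraTrack is a spline track actor for the bubble-jumping game that guides the camera and seeds level generation.
; On BeginPlay it registers itself on the game state, caches the player pawn, and hands its spline to the level generator to spawn bouncers.
; Helper functions return the spline point nearest the player and the spline's world rotation at a given location for camera orientation.
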(event EventBeginPlay
  (Variables|/Game/MegaJam/Blueprint/GameData/GameState_BubbleJumping.GameState_BubbleJumping_C|SetCameraTrack (.AsGame%20State%20Bubble%20Jumping (Utilities|Casting|CastToGameState_BubbleJumping (Game|GetGameState))) self)
  (Variables|Default|SetPlayerPawn (Game|Player|GetPlayerPawn 0))
  (Variables|/Game/MegaJam/Blueprint/Level/BP_LevelGenerator.BP_LevelGenerator_C|SetSpline (Variables|Default|GetBP_LevelGenerator) (Variables|Default|GetSpline))
  (Default|GenerateBouncer (Variables|Default|GetBP_LevelGenerator)))

(event EventTick
  (params (DeltaSeconds :type Float%20%28single-precision%29)))

(fn ConstructionScript)

(fn GetPlayerLocationonTrack
  (return (Spline|FindLocationClosesttoWorldLocation (Variables|Default|GetSpline) (Transformation|GetActorLocation (Variables|Default|GetPlayerPawn)) "World")))

(fn GetCameraRotation
  (params (WorldSplineLocation :type Vector%20%28by%20ref%29) (Jumper :type BP%20Bubble%20Jumper%20Character%20Object%20Reference))
  (bind _spline (Variables|Default|GetSpline))
  (if (Variables|/Game/MegaJam/Blueprint/Character/BP_BubbleJumperCharacter.BP_BubbleJumperCharacter_C|GetImpulsing Jumper)
    _
    (else
      _))
  (return (Class|SplineComponent|GetRotationatSplineInputKey _spline (Class|SplineComponent|FindInputKeyClosesttoWorldLocation _spline WorldSplineLocation) "World")))