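; Test bubble actor that bounces overlapping characters and other objects away from its center.
; On CollisionDetector begin overlap, the launch velocity is the offset from the detector to the other actor, scaled by a constant.
; Characters have their velocity zeroed before LaunchCharacter, and a debug line shows the launch vector.
; Anything else has the overlapped component's physics linear velocity replaced with that vector.
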(event OnComponentBeginOverlap(collisionDetector)
  (params (OverlappedComponent :type Primitive%20Component%20Object%20Reference) (OtherActor :type Actor%20Object%20Reference) (OtherComp :type Primitive%20Component%20Object%20Reference) (OtherBodyIndex :type Integer) (bFromSweep :type Boolean) (SweepResult :type Hit%20Result%20Structure%20%28by%20ref%29))
  (bind _returnvalue (Transformation|GetActorLocation OtherActor))
  (bind _collisiondetector (Variables|Default|GetcollisionDetector))
  (bind _returnvalue_2 (Transformation|GetWorldLocation _collisiondetector))
  (bind _returnvalue_3 (- _returnvalue _returnvalue_2))
  (bind _returnvalue_4 (* _returnvalue_3 3.0))
  (Variables|Default|Setforce _returnvalue_4)
  (bind _ascharacter (Utilities|Casting|CastToCharacter OtherActor)
    (:then
      (Variables|/Script/Engine.MovementComponent|SetVelocity (Pawn|GetMovementComponent _ascharacter) "0, 0, 0")
      (Character|LaunchCharacter _ascharacter (Variables|Default|Getforce) false false)
      (Rendering|Debug|DrawDebugLine _returnvalue (+ _returnvalue _returnvalue_4) "(R=0.000000,G=0.000000,B=0.000000,A=1.000000)" 5.0 0.0))
    (:CastFailed
      (Physics|SetPhysicsLinearVelocity OtherComp (Variables|Default|Getforce) false "None"))))

(event OnComponentHit(collisionDetector)
  (params (HitComponent :type Primitive%20Component%20Object%20Reference) (OtherActor :type Actor%20Object%20Reference) (OtherComp :type Primitive%20Component%20Object%20Reference) (NormalImpulse :type Vector :default "0, 0, 0") (Hit :type Hit%20Result%20Structure%20%28by%20ref%29)))

(event EventBeginPlay)

(event Collision|EventActorBeginOverlap
  (params (OtherActor :type Actor%20Object%20Reference)))

(event EventTick
  (params (DeltaSeconds :type Float%20%28single-precision%29)))

(fn ConstructionScript)