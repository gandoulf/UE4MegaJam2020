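; Bubble bouncer that repels overlapping objects and handles the bubble jumper character's bounces.
; On overlap, a trace toward its detector yields a fixed-strength outward force, applied directly as velocity to non-character components.
; For the character it calls StartBounce and rotates each tick around an axis derived from the character and an offset spline point's direction.
; StopBouncing recomputes the force and disables tick; spline lookup code is disconnected.
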(event OnComponentBeginOverlap(collisionDetector)
  (params (OverlappedComponent :type Primitive%20Component%20Object%20Reference) (OtherActor :type Actor%20Object%20Reference) (OtherComp :type Primitive%20Component%20Object%20Reference) (OtherBodyIndex :type Integer) (bFromSweep :type Boolean) (SweepResult :type Hit%20Result%20Structure%20%28by%20ref%29))
  (bind _spline (Variables|Default|GetSpline))
  (CallFunction|ComputeForce OtherActor)
  (bind _asbp_bubble_jumper_character (Utilities|Casting|CastToBP_BubbleJumperCharacter OtherActor)
    (:then
      (bind _output_get (Variables|Default|SetBubble%20Jumper%20Character _asbp_bubble_jumper_character))
      (Default|StartBounce _output_get self)
      (Variables|Default|SetBouncing true)
      (Rendering|Debug|DrawDebugSphere (Spline|GetLocationatTime _spline (+ (Variables|Default|GetSplineTime) (/ (Variables|setting|GetBounceSplineDistOffset) (Spline|GetSplineLength _spline))) "World" true) 1e+02 12 "(R=1.000000,G=0.000000,B=0.000000,A=1.000000)" 5.0 3.0)
      (Actor|Tick|SetActorTickEnabled true))
    (:CastFailed
      (Physics|SetPhysicsLinearVelocity OtherComp (Variables|Default|Getforce) false "None"))))

(event Custom|StopBouncing
  (CallFunction|ComputeForce (Variables|Default|GetBubble%20Jumper%20Character))
  (Variables|Default|SetBouncing false)
  (Actor|Tick|SetActorTickEnabled false)
  (Variables|Default|SetBubble%20Jumper%20Character 0))

(event Custom|InitBouncer
  (bind _spline (Variables|Default|GetSpline))
  (Variables|Default|SetRotationDir (Math|Vector|Normalize (- (Spline|GetLocationatTime _spline (+ (Variables|Default|GetSplineTime) (/ (Variables|setting|GetBounceSplineDistOffset) (Spline|GetSplineLength _spline))) "World" true) (Transformation|GetActorLocation)))))

(event EventTick
  (params (DeltaSeconds :type Float%20%28single-precision%29))
  (CallFunction|OrientateBouncer))

(event EventBeginPlay
  (Variables|Default|GetSpline
    (:then
      (CallFunction|InitBouncer))
    (:else)))

(fn ConstructionScript)

(fn ComputeForce
  (params (ActorCollided :type Actor%20Object%20Reference))
  (bind _returnvalue (Transformation|GetActorLocation ActorCollided))
  (bind _outhit (Collision|LineTraceByChannel _returnvalue (Transformation|GetWorldLocation (Variables|Default|GetcollisionDetector)) "TraceTypeQuery1" false 0 "ForDuration" false))
  (if true
    (Variables|Default|Setforce (* (Math|Vector|Normalize (- _returnvalue (.location _outhit))) 1e+03))))

(fn OrientateBouncer
  (if (Variables|Default|GetBouncing)
    (bind _bubble_jumper_character (Variables|Default|GetBubble%20Jumper%20Character)
      (:then
        (Class|Actor|AddActorWorldRotation (Math|Vector|RotatorfromAxisandAngle (Math|Vector|CrossProduct (- (Transformation|GetActorLocation _bubble_jumper_character) (Transformation|GetActorLocation)) (Variables|Default|GetRotationDir)) 2.0)))
      (:else))))