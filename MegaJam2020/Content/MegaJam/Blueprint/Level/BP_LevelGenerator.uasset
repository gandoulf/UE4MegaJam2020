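; Level generator that scatters randomly chosen bouncer actors along a spline.
; GenerateBouncer steps along the spline in fixed-distance segments, spawning a randomised number of bouncers at random offsets in each.
; SpawnBouncer pushes each one out perpendicular to the spline at a random angle and distance, with random per-axis scale, forming a tube-like field.
; BeginPlay is empty, so nothing in this graph triggers generation.
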(event EventBeginPlay)

(fn GenerateBouncer
  (bind _spline (Variables|Default|GetSpline))
  (bind _bouncerdancitynum (Variables|Default|GetBouncerDancityNum))
  (bind _returnvalue (Spline|GetSplineLength _spline))
  (bind _returnvalue_2 (Math|Float|Truncate (.x _bouncerdancitynum)))
  (LocalVariables|SetSplineDist _returnvalue)
  (LocalVariables|SetDincityDistTime (/ (Variables|Default|GetBouncerDancityDist) _returnvalue))
  (while (< (LocalVariables|GetSplineTime) 1.0)
    (for _index (range _returnvalue_2 (Math|Random|RandomIntegerinRange _returnvalue_2 (Math|Float|Truncate (.y _bouncerdancitynum))))
      (CallFunction|SpawnBouncer (+ (LocalVariables|GetSplineTime) (/ (Math|Random|RandomFloatinRange 0.0 (Variables|Default|GetBouncerDancityDist)) (LocalVariables|GetSplineDist)))))
    (LocalVariables|SetSplineTime (+ (LocalVariables|GetSplineTime) (LocalVariables|GetDincityDistTime)))))

(fn SpawnBouncer
  (params (SplineTime :type Float%20%28single-precision%29))
  (bind _returnvalue (Math|Random|RandomFloatinRange 2.0 4.0))
  (bind _distancefromspline (Variables|Default|GetDistanceFromSpline))
  (bind _spline (Variables|Default|GetSpline))
  (bind _returnvalue_2 (Class|SplineComponent|GetDirectionatTime _spline SplineTime "Local" false))
  (Game|SpawnActorfromClass (.OutItem (Utilities|Array|Random (Variables|Default|GetBouncerClass))) (Math|Transform|MakeTransform (+ (Spline|GetLocationatTime (Variables|Default|GetSpline) SplineTime "World" false) (* (Math|Vector|RotateVectorAroundAxis (Math|Vector|CrossProduct (Class|SplineComponent|GetUpVectoratTime _spline SplineTime "Local" false) _returnvalue_2) (Math|Random|RandomFloatinRange 0.0 3.6e+02) _returnvalue_2) (Math|Random|RandomFloatinRange (.x _distancefromspline) (.y _distancefromspline)))) "0, 0, 0" (Math|Vector|MakeVector _returnvalue _returnvalue _returnvalue)) "AdjustIfPossibleButAlwaysSpawn" 0 0))