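; BP_StartingPoint is the bubble the player character sits on at the start, until launched along an arrow.
; BeginPlay creates the main menu and runs SetUpPlayer, which pins the character at the arrow, disables its movement and physics, and feeds dent position and normal into the sphere's dynamic material.
; Tick keeps the character oriented outward from the sphere.
; ThrowCharacter plays the jump animation, launches after a short delay, restores control and clears widgets on first throw.
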(event Custom|SetUpPlayer
  (bind _startpointmaterial (Variables|Default|GetStartPointMaterial))
  (bind _bubble_jumper_character (Variables|Default|GetBubble%20Jumper%20Character))
  (bind _bubble_jumper_character_2 (Variables|Default|GetBubble%20Jumper%20Character))
  (bind _bubble_jumper_character_3 (Variables|Default|GetBubble%20Jumper%20Character))
  (bind _mesh (Variables|/Script/Engine.Character|GetMesh _bubble_jumper_character_2))
  (Rendering|Material|SetVectorParameterValue _startpointmaterial "position" (Math|Conversions|ToLinearColor(Vector) (Transformation|GetWorldLocation (Variables|Default|GetArrow))) :!class /Script/Engine.MaterialInstanceDynamic)
  (Rendering|Material|SetVectorParameterValue _startpointmaterial "Normal" (Math|Conversions|ToLinearColor(Vector) (* (Math|Vector|Normalize (- (Transformation|GetWorldLocation (Variables|Default|GetArrow)) (Transformation|GetActorLocation))) (* -1.0 (Variables|Default|GetBounceIntencity) (.x (Transformation|GetActorScale3D))))) :!class /Script/Engine.MaterialInstanceDynamic)
  (Transformation|SetActorLocation _bubble_jumper_character (Transformation|GetWorldLocation (Variables|Default|GetArrow)) false false)
  (Default|EnableMouvement _bubble_jumper_character false self)
  (Variables|/Script/Engine.MovementComponent|SetVelocity (Pawn|GetMovementComponent _bubble_jumper_character) "0, 0, 0")
  (Default|EnablePhysics _bubble_jumper_character false)
  (Variables|Default|SetPlayerOnStartPoint true)
  (Transformation|SetActorRotation _bubble_jumper_character_3 (Math|Rotator|MakeRotfromZX (Math|Vector|GetForwardVector (Math|Rotator|FindLookatRotation (Transformation|GetActorLocation) (Transformation|GetActorLocation _bubble_jumper_character_3))) (Transformation|GetActorForwardVector _bubble_jumper_character_3)))
  ;[1 1 1] set relativeLoc
  (Transformation|SetRelativeLocation _mesh (+ "0, 0,-95.000000" (* (Math|Vector|MakeVector 0.0 0.0 -25.0) (.x (Transformation|GetActorScale3D)))) false false)
  (bind _aschara_anim_blueprint (Utilities|Casting|CastToChara_AnimBlueprint (Components|SkeletalMesh|GetAnimInstance _mesh)))
  (Default|Landing _aschara_anim_blueprint))

(event Custom|ThrowCharacter
  (bind _bubble_jumper_character (Variables|Default|GetBubble%20Jumper%20Character))
  (bind _bubble_jumper_character_2 (Variables|Default|GetBubble%20Jumper%20Character))
  (if (Variables|Default|GetPlayerOnStartPoint)
    (bind _aschara_anim_blueprint (Utilities|Casting|CastToChara_AnimBlueprint (Components|SkeletalMesh|GetAnimInstance (Variables|/Script/Engine.Character|GetMesh (Variables|Default|GetBubble%20Jumper%20Character)))))
    (Default|InJump _aschara_anim_blueprint)
    (Utilities|FlowControl|Delay 0.15)
    (Character|LaunchCharacter _bubble_jumper_character (* (Math|Vector|GetForwardVector (Variables|Default|GetArrow)) 1.5e+03) false false)
    (Transformation|SetWorldRotation (Variables|/Script/Engine.Character|GetCapsuleComponent _bubble_jumper_character) "0, 0, 0" false false)
    (Default|EnableMouvement _bubble_jumper_character_2 true self)
    (Default|EnablePhysics _bubble_jumper_character_2 true)
    (Variables|Default|SetPlayerOnStartPoint false)
    (Transformation|SetRelativeLocation (Variables|/Script/Engine.Character|GetMesh (Variables|Default|GetBubble%20Jumper%20Character)) "0, 0,-95.000000" false false)
    (if (not (Variables|Default|GetGameAsStart))
      (Viewport|RemoveAllWidgets)
      (Variables|Default|SetGameAsStart true))))

(event EventBeginPlay
  (bind _returnvalue (Rendering|Material|CreateDynamicMaterialInstance "/Game/Art/Texture/Bounce/MI_Ball_Player.MI_Ball_Player" "None" "None" :!class /Script/Engine.KismetMaterialLibrary))
  (bind _output_get (Variables|Default|SetStartPointMaterial _returnvalue))
  (Rendering|Material|SetMaterial (Variables|Default|GetSphere) 0 _output_get)
  (bind _asbp_bubble_jumper_character (Utilities|Casting|CastToBP_BubbleJumperCharacter (Game|Player|GetPlayerPawn 0)))
  (Variables|Default|SetBubble%20Jumper%20Character _asbp_bubble_jumper_character)
  (CallFunction|SetUpPlayer)
  (bind _returnvalue_2 (UserInterface|CreateWidget "/Game/MegaJam/Blueprint/GUI/WBP_MainMenu.WBP_MainMenu_C"))
  (UserInterface|Viewport|AddtoViewport _returnvalue_2 0))

(event EventTick
  (params (DeltaSeconds :type Float%20%28single-precision%29))
  (bind _bubble_jumper_character (Variables|Default|GetBubble%20Jumper%20Character))
  (if (Variables|Default|GetPlayerOnStartPoint)
    (Transformation|SetActorRotation _bubble_jumper_character (Math|Rotator|MakeRotfromZX (Math|Vector|GetForwardVector (Math|Rotator|FindLookatRotation (Transformation|GetActorLocation) (Transformation|GetActorLocation _bubble_jumper_character))) (Transformation|GetActorForwardVector _bubble_jumper_character)))))

(fn ConstructionScript)