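; Actor component that predicts the owning character's flight path each tick to detect a BouncingBubble ahead.
; It samples position and velocity, then builds a gravity-adjusted arc of short segments over a set number of prediction steps.
; Each segment is debug-drawn and line-traced until a hit; a BouncingBubble hit sets BouncerDetected.
; Capsule tracing, IDodger dodge calls and landing-marker placement are left disconnected, and SetDecalVisibility is empty.
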(event EventBeginPlay
  (bind _asbp_bubble_jumper_character (Utilities|Casting|CastToBP_BubbleJumperCharacter (Components|GetOwner)))
  (Variables|Default|SetBubble%20Jumper%20Character _asbp_bubble_jumper_character))

(event EventTick
  (params (DeltaSeconds :type Float%20%28single-precision%29))
  (bind _returnvalue (Components|GetOwner))
  (bind _ascharacter (Utilities|Casting|CastToCharacter _returnvalue))
  (bind _returnvalue_2 (Pawn|GetMovementComponent _ascharacter))
  (Variables|Default|SetBouncerDetected false)
  (Utilities|FlowControl|Sequence
    (:then_0
      (Variables|Default|Setmovement _returnvalue_2)
      (Variables|Default|Setplayer_velocity (Variables|/Script/Engine.MovementComponent|GetVelocity _returnvalue_2))
      (Variables|Default|Setplayer_position (Transformation|GetActorLocation _ascharacter)))
    (:then_1
      (Utilities|Array|SetArrayElem (Variables|Default|Gettrace_start_points) 0 (Variables|Default|Getplayer_position) true)
      (Utilities|Array|SetArrayElem (Variables|Default|Gettrace_vectors) 0 (* (Variables|Default|Getplayer_velocity) (Variables|Default|Getprediction_tick_time)) true)
      (bind _index (Utilities|FlowControl|ForLoopwithBreak 1 (Variables|Default|Getprediction_ticks))
        (:LoopBody
          (Utilities|Array|SetArrayElem (Variables|Default|Gettrace_start_points) _index (+ (Utilities|Array|Get(acopy) (Variables|Default|Gettrace_vectors) (- _index 1)) (Utilities|Array|Get(acopy) (Variables|Default|Gettrace_start_points) (- _index 1))) true)
          (Utilities|Array|SetArrayElem (Variables|Default|Gettrace_vectors) _index (Math|Vector|MakeVector (.X (Math|Vector|BreakVector (Utilities|Array|Get(acopy) (Variables|Default|Gettrace_vectors) (- _index 1)))) (.Y (Math|Vector|BreakVector (Utilities|Array|Get(acopy) (Variables|Default|Gettrace_vectors) (- _index 1)))) (+ (* (Variables|Default|Getprediction_tick_time) (* (Variables|Default|Getprediction_tick_time) (Components|Movement|GetGravityZ (Variables|Default|Getmovement)))) (.Z (Math|Vector|BreakVector (Utilities|Array|Get(acopy) (Variables|Default|Gettrace_vectors) (- _index 1)))))) true))
        (:Completed
          (bind _index_2 (Utilities|FlowControl|ForLoopwithBreak 0 (Variables|Default|Getprediction_ticks) :!label _label)
            (:LoopBody
              (Rendering|Debug|DrawDebugLine (Utilities|Array|Get(acopy) (Variables|Default|Gettrace_start_points) _index_2) (+ (Utilities|Array|Get(acopy) (Variables|Default|Gettrace_start_points) _index_2) (Utilities|Array|Get(acopy) (Variables|Default|Gettrace_vectors) _index_2)) "(R=0.116624,G=0.000000,B=1.000000,A=1.000000)" 0.1 0.0)
              (bind (_outhit _returnvalue_3) (Collision|LineTraceByChannel (Utilities|Array|Get(acopy) (Variables|Default|Gettrace_start_points) _index_2) (+ (Utilities|Array|Get(acopy) (Variables|Default|Gettrace_start_points) _index_2) (Utilities|Array|Get(acopy) (Variables|Default|Gettrace_vectors) _index_2)) "TraceTypeQuery1" false 0 "None" true "(R=1.000000,G=0.000000,B=0.000000,A=1.000000)" "(R=0.000000,G=1.000000,B=0.000000,A=1.000000)" 0.1))
              (if _returnvalue_3
                (Utilities|Casting|CastToBouncingBubble (.HitActor (Collision|BreakHitResult _outhit)))
                (Variables|Default|SetBouncerDetected true)
                (goto _label Break)))))))))