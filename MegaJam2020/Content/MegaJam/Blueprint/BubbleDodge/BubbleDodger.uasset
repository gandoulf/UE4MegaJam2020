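; BubbleDodger is a component that decides whether its owner should dodge an incoming impact and tracks the dodge state.
; Dodge accepts impacts within a maximum duration whose direction aligns closely enough with the surface normal from a trace toward the impact point.
; It stores the latest target, position and duration, starting a dodge if none is active.
; Movement looks unfinished: Tick pins the owner to world origin while dodging, and nothing here calls StopDodge.
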(event EventBeginPlay)

(event EventTick
  (params (DeltaSeconds :type Float%20%28single-precision%29))
  (if (Variables|Default|Getis_dodging)
    (Transformation|SetWorldLocation (Variables|/Script/Engine.Actor|GetRootComponent (Components|GetOwner)) "0, 0, 0" false false)))

(fn Dodge
  (params (player :type Actor%20Object%20Reference) (impact_position :type Vector :default "0, 0, 0") (impact_direction :type Vector :default "0, 0, 0") (dodge_duration :type Float%20%28single-precision%29))
  (|CallParentFunction player impact_position impact_direction dodge_duration)
  (bind _should_dodge (CallFunction|ShouldDodge impact_position impact_direction dodge_duration))
  (if _should_dodge
    (Variables|Default|Setcurrent_dodge_target player)
    (Variables|Default|Setcurrent_dodge_position impact_position)
    (Variables|Default|Setcurrent_dodge_duration dodge_duration)
    (if (not (Variables|Default|Getis_dodging))
      (CallFunction|StartDodge))))

(fn ShouldDodge
  (params (dodge_position :type Vector) (dodge_direction :type Vector) (dodge_duration :type Float%20%28single-precision%29))
  (if (<= dodge_duration (Variables|Default|Getdodge_max_duration))
    (bind (_outhit _returnvalue) (Collision|LineTraceByChannel (Transformation|GetWorldLocation (Variables|/Script/Engine.Actor|GetRootComponent (Components|GetOwner))) dodge_position "TraceTypeQuery1" false 0 "None" false))
    (Development|PrintString "Could not find collision" (not _returnvalue) (not _returnvalue) "(R=1.000000,G=0.018510,B=0.000000,A=1.000000)" 1.0)
    (return (> (Math|Float|Absolute(Float) (Math|Vector|DotProduct (Math|Vector|Normalize dodge_direction) (Math|Vector|Normalize (.Normal (Collision|BreakHitResult _outhit))))) (Variables|Default|Getdodge_threshold)))
    (else
      (return false))))

(fn StartDodge
  (Development|PrintString "Dodging")
  (Variables|Default|Setcurrent_dodge_start_time (Utilities|Time|GetTimeSeconds))
  (Variables|Default|Setis_dodging true))

(fn StopDodge
  (Variables|Default|Setis_dodging false))